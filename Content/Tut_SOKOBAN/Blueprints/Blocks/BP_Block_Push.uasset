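; BP_Block_Push is a pushable block for a Sokoban tutorial game that slides one box length in a requested direction.
; TryMoveTo line-traces on the Visibility channel from its location to the target, returning false if blocked, or starting the move timeline and returning true.
; The timeline's update eases the actor between the stored start and goal locations without sweeping.
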(event EventBeginPlay
  (|CallParentFunction) ; This node is disabled and will not be called.\nDrag off pins to build functionality.
)

(event Collision|EventActorBeginOverlap
  (params (OtherActor :type Actor%20Object%20Reference))
  (|CallParentFunction OtherActor) ; This node is disabled and will not be called.\nDrag off pins to build functionality.
)

(event EventTick
  (params (DeltaSeconds :type Float%20%28single-precision%29))
  (|CallParentFunction DeltaSeconds) ; This node is disabled and will not be called.\nDrag off pins to build functionality.
)

(fn ConstructionScript
  (|CallParentFunction))

(fn TryMoveto
  (params (Dir :type Vector%202D%20Structure))
  (bind _returnvalue (Transformation|GetActorLocation))
  (bind _return (Utilities|BoxEdgeLength))
  (Variables|Default|SetStartLoc _returnvalue)
  (Variables|Default|SetGoalLoc (+ _returnvalue (* Dir (Math|Vector2D|MakeVector2D _return _return))))
  (bind _returnvalue_2 (Collision|LineTraceByChannel (Variables|Default|GetStartLoc) (Variables|Default|GetGoalLoc) "TraceTypeQuery1" false 0 "None"))
  (if (not _returnvalue_2)
    (Components|Timeline|PlayfromStart (Variables|Default|GetTimeline_Move))
    (return true)
    (else
      (return false))))