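; Player controller for a Sokoban tutorial that moves the controlled pawn in box-sized steps.
; On BeginPlay it adds the IMC_Move Enhanced Input mapping context.
; Each IA_Move trigger offsets the pawn by the 2D input scaled by BoxEdgeLength and turns it to face that direction.
; Location is set directly without sweep, so this controller performs no collision or push checks.
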(event Input|EnhancedActionEvents|EnhancedInputActionIA_Move
  (params (ActionValue :type Vector%202D%20Structure) (ElapsedSeconds :type Float%20%28double-precision%29) (TriggeredSeconds :type Float%20%28double-precision%29) (InputAction :type Input%20Action%20Object%20Reference :default "/Game/Tut_SOKOBAN/Inputs/IA_Move.IA_Move"))
  (bind _returnvalue (Pawn|GetControlledPawn))
  (bind (_x _y) (Math|Vector2D|BreakVector2D ActionValue))
  (bind _return (Utilities|BoxEdgeLength))
  (:Triggered
    (Transformation|SetActorLocation _returnvalue (+ (Transformation|GetActorLocation _returnvalue) (* ActionValue (Math|Vector2D|MakeVector2D _return _return))) false false)
    (Transformation|SetActorRotation (Pawn|GetControlledPawn) (Math|Rotator|MakeRotfromX (Math|Vector|MakeVector _x _y 0.0)))))

(event EventBeginPlay
  (Input|AddMappingContext (PlayerController|LocalPlayerSubsystems|GetEnhancedInputLocalPlayerSubsystem) "/Game/Tut_SOKOBAN/Inputs/IMC_Move.IMC_Move" 0 "(bIgnoreAllPressedKeysUntilRelease=True,bForceImmediately=False)"))

(fn ConstructionScript)