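; Stage builder actor for the Sokoban game that spawns a level from a Paper2D tile map when play begins.
; It reads the StageName URL option, finds the map in DT_StageAssetPath, and loads it synchronously.
; Each tile index spawns a wall, pushable block, goal, or player, which gets possessed.
; It then moves the camera over the map's center and gives GM_GamePlay the goal count.
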(event Custom|BuildStage
  (params (Target :type Paper%20Tile%20Map%20Object%20Reference))
  (bind _return (Utilities|BoxEdgeLength))
  (bind _return_2 (Utilities|BoxEdgeLength))
  (bind _papertilemap (Variables|Default|GetPaperTileMap))
  (bind _returnvalue (/ _return 2.0))
  ;[1 1 1] ステージを構築.
  (Class|PaperTileMapComponent|SetTileMap _papertilemap Target)
  (bind (_mapwidth _mapheight) (Class|PaperTileMapComponent|GetMapSize _papertilemap))
  (for _index (range 0 (- _mapheight 1)) ; Row
    (for _index_2 (range 0 (- _mapwidth 1)) ; Col
      (switch int (.TileIndex (Class|TileMapBlueprintLibrary|BreakTile (Class|PaperTileMapComponent|GetTile (Variables|Default|GetPaperTileMap) _index_2 _index)))
        (:1
          (Game|SpawnActorfromClass "/Game/Tut_SOKOBAN/Blueprints/Blocks/BP_Block_Wall.BP_Block_Wall_C" (Math|Transform|MakeTransform (Math|Vector|MakeVector (* _index_2 _return_2) (* _index _return_2) 5e+01) "0, 0, 0" "1.000000,1.000000,1.000000") "Undefined" 0 0))
        (:2
          (Game|SpawnActorfromClass "/Game/Tut_SOKOBAN/Blueprints/Blocks/BP_Block_Push.BP_Block_Push_C" (Math|Transform|MakeTransform (Math|Vector|MakeVector (* _index_2 _return_2) (* _index _return_2) 5e+01) "0, 0, 0" "1.000000,1.000000,1.000000") "Undefined" 0 0))
        (:3
          (Game|SpawnActorfromClass "/Game/Tut_SOKOBAN/Blueprints/Blocks/BP_Block_Goal.BP_Block_Goal_C" (Math|Transform|MakeTransform (Math|Vector|MakeVector (* _index_2 _return_2) (* _index _return_2) 5e+01) "0, 0, 0" "1.000000,1.000000,1.000000") "Undefined" 0 0)
          (Math|Integer|IncrementInt (Variables|Default|GetNumGoalBlock)))
        (:4
          (bind _returnvalue_2 (Game|SpawnActorfromClass "/Game/Tut_SOKOBAN/Blueprints/Player/BP_Player.BP_Player_C" (Math|Transform|MakeTransform (Math|Vector|MakeVector (* _index_2 _return_2) (* _index _return_2) 5e+01) "0, 0, 0" "1.000000,1.000000,1.000000") "Undefined" 0 0))
          (Pawn|Possess (Game|GetPlayerController 0) _returnvalue_2)))))
  (Transformation|SetActorLocation (Variables|Default|GetCameraActor) (Math|Vector|MakeVector (* _mapwidth _returnvalue) (* _mapheight _returnvalue) 1e+03) false false)
  (Variables|/Game/Tut_SOKOBAN/Blueprints/GM_GamePlay.GM_GamePlay_C|SetTargetNumGoalBlock (.AsGM%20Game%20Play (Utilities|Casting|CastToGM_GamePlay (Game|GetGameMode))) (Variables|Default|GetNumGoalBlock)))

(event EventBeginPlay
  ;[1 1 1] ステージデータをロード.
  (bind _returnvalue (Utilities|GetDataTableRow "/Game/Tut_SOKOBAN/Blueprints/StageBuilder/DT_StageAssetPath.DT_StageAssetPath" (Utilities|String|StringToName (Class|GameplayStatics|ParseOption (Variables|/Script/Engine.GameModeBase|GetOptionsString (Game|GetGameMode)) "StageName"))) ; Get Data Table Rowノード.
    (:then
      (bind _returnvalue_2 (Utilities|LoadAssetBlocking (Utilities|Struct|BreakSStageAssetPath _returnvalue)))
      (bind _aspaper_tile_map (Utilities|Casting|CastToPaperTileMap _returnvalue_2)
        (:then
          (CallFunction|BuildStage _aspaper_tile_map))
        (:CastFailed
          (Development|PrintString "ERROR : Paper Tile Mapへのキャストに失敗."))))
    (:RowNotFound
      (Development|PrintString "ERROR : ステージデータがありません."))))

(fn ConstructionScript)